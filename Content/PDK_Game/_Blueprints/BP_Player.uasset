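; Top-down 2D player pawn with Enhanced Input movement, four-way flipbook animation and interaction.
; Movement input sets facing and moving state, which Tick uses to pick walk or idle flipbooks, rotating one side-facing set for left and right.
; Interact box-overlaps a facing-rotated zone for BPI_InteractableObject actors, with optional debug drawing.
; IsInDialogue reads inverted: true allows movement and interaction, while false makes Interact fire the dialogue-continue dispatcher.
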(event Input|EnhancedActionEvents|EnhancedInputActionIA_Interact
  (params (ActionValue :type Boolean) (ElapsedSeconds :type Float%20%28double-precision%29) (TriggeredSeconds :type Float%20%28double-precision%29) (InputAction :type Input%20Action%20Object%20Reference :default "/Game/PDK_Game/Input/Actions/IA_Interact.IA_Interact"))
  ;[1 1 1] Interaction
  (:Started
    (if (Variables|Default|GetisInDialogue)
      (CallFunction|Interact)
      (else
        (Default|CallOnDialogueContinue)))))

(event Input|EnhancedActionEvents|EnhancedInputActionIA_MoveHorizontal
  (params (ActionValue :type Float%20%28double-precision%29) (ElapsedSeconds :type Float%20%28double-precision%29) (TriggeredSeconds :type Float%20%28double-precision%29) (InputAction :type Input%20Action%20Object%20Reference :default "/Game/PDK_Game/Input/Actions/IA_MoveHorizontal.IA_MoveHorizontal"))
  ;[1 1 1] Movement
  (:Triggered
    (if (Variables|Default|GetisInDialogue) :!label _label
      (Pawn|Input|AddMovementInput "1.000000,0.000000,0.000000" ActionValue false)
      (Variables|Default|SetisMoving (or (!= ActionValue 0.0) (!= 0.0 (stale Input|EnhancedActionEvents|EnhancedInputActionIA_MoveVertical ActionValue))))
      (CallFunction|HandleDirection ActionValue (stale Input|EnhancedActionEvents|EnhancedInputActionIA_MoveVertical ActionValue))))
  (:Completed
    (goto _label)))

(event Input|EnhancedActionEvents|EnhancedInputActionIA_MoveVertical
  (params (ActionValue :type Float%20%28double-precision%29) (ElapsedSeconds :type Float%20%28double-precision%29) (TriggeredSeconds :type Float%20%28double-precision%29) (InputAction :type Input%20Action%20Object%20Reference :default "/Game/PDK_Game/Input/Actions/IA_MoveVertical.IA_MoveVertical"))
  ;[1 1 1] Movement
  (:Triggered
    (if (Variables|Default|GetisInDialogue) :!label _label
      (Pawn|Input|AddMovementInput "0.000000,1.000000,0.000000" ActionValue false)
      (Variables|Default|SetisMoving (or (!= (stale Input|EnhancedActionEvents|EnhancedInputActionIA_MoveHorizontal ActionValue) 0.0) (!= 0.0 ActionValue)))
      (CallFunction|HandleDirection (stale Input|EnhancedActionEvents|EnhancedInputActionIA_MoveHorizontal ActionValue) ActionValue)))
  (:Completed
    (goto _label)))

(event EventBeginPlay
  ;[1 1 1] Input Setup
  (bind _asplayer_controller (Utilities|Casting|CastToPlayerController (Pawn|GetController)))
  (Input|AddMappingContext (PlayerController|LocalPlayerSubsystems|GetEnhancedInputLocalPlayerSubsystem _asplayer_controller) "/Game/PDK_Game/Input/IMC_TopDown.IMC_TopDown" 0 "(bIgnoreAllPressedKeysUntilRelease=True,bForceImmediately=False,bNotifyUserSettings=False)"))

(event EventTick
  (params (DeltaSeconds :type Float%20%28single-precision%29))
  ;[1 1 1] Update Loop
  (CallFunction|HandleAnimation)
  (CallFunction|DrawInteractZone))

(fn ConstructionScript)

(fn HandleDirection
  (params (horizontalInput :type Float%20%28double-precision%29) (verticalInput :type Float%20%28double-precision%29))
  (if (> verticalInput 0.0)
    (Variables|Default|Setdirection "NewEnumerator3")
    (elif (< verticalInput 0.0)
      (Variables|Default|Setdirection "NewEnumerator2")
      (elif (> horizontalInput 0.0)
        (Variables|Default|Setdirection "NewEnumerator0")
        (elif (< horizontalInput 0.0)
          (Variables|Default|Setdirection "NewEnumerator1"))))))

(fn HandleAnimation
  (bind _sprite (Variables|Default|GetSprite))
  (bind _sprite_2 (Variables|Default|GetSprite))
  (if (Variables|Default|GetisMoving)
    (switch Utilities|FlowControl|Switch|SwitchonEN_PlayerDirection (Variables|Default|Getdirection)
      (:NewEnumerator0
        (Sprite|SetFlipbook _sprite_2 "/Game/PDK_Game/Sprites/Tests/Flipbooks/FL_leader/FL_leader_walkRight.FL_leader_walkRight")
        (CallFunction|SetSpriteRotation true))
      (:NewEnumerator1
        (Sprite|SetFlipbook _sprite_2 "/Game/PDK_Game/Sprites/Tests/Flipbooks/FL_leader/FL_leader_walkRight.FL_leader_walkRight")
        (CallFunction|SetSpriteRotation false))
      (:NewEnumerator2
        (Sprite|SetFlipbook _sprite_2 "/Game/PDK_Game/Sprites/Tests/Flipbooks/FL_leader/FL_leader_walkUp.FL_leader_walkUp"))
      (:NewEnumerator3
        (Sprite|SetFlipbook _sprite_2 "/Game/PDK_Game/Sprites/Tests/Flipbooks/FL_leader/FL_leader_walkDown.FL_leader_walkDown")))
    (else
      (switch Utilities|FlowControl|Switch|SwitchonEN_PlayerDirection (Variables|Default|Getdirection)
        (:NewEnumerator0
          (Sprite|SetFlipbook _sprite "/Game/PDK_Game/Sprites/Tests/Flipbooks/FL_leader/FL_leader_idleRight.FL_leader_idleRight")
          (CallFunction|SetSpriteRotation true))
        (:NewEnumerator1
          (Sprite|SetFlipbook _sprite "/Game/PDK_Game/Sprites/Tests/Flipbooks/FL_leader/FL_leader_idleRight.FL_leader_idleRight")
          (CallFunction|SetSpriteRotation false))
        (:NewEnumerator2
          (Sprite|SetFlipbook _sprite "/Game/PDK_Game/Sprites/Tests/Flipbooks/FL_leader/FL_leader_idleUp.FL_leader_idleUp"))
        (:NewEnumerator3
          (Sprite|SetFlipbook _sprite "/Game/PDK_Game/Sprites/Tests/Flipbooks/FL_leader/FL_leader_idleDown.FL_leader_idleDown"))))))

(fn SetSpriteRotation
  (params (right :type Boolean))
  (bind _sprite (Variables|Default|GetSprite))
  (if right
    (Transformation|SetRelativeRotation _sprite (Math|Rotator|MakeRotator -3e+01 0.0 0.0) false false)
    (else
      (Transformation|SetRelativeRotation _sprite (Math|Rotator|MakeRotator 3e+01 0.0 1.8e+02) false false))))

(fn Interact
  (bind _result (CallFunction|GetInteractZoneTransform))
  (bind _outactors (Collision|BoxOverlapActors (.location _result) (.scale _result) (Utilities|Array|MakeArray "ObjectTypeQuery1") 0 :!class /Script/Engine.KismetSystemLibrary))
  (for _array_element _outactors
    (bind _asbpi_interactable_object (Utilities|Casting|CastToBPI_InteractableObject _array_element))
    (Default|Interact _asbpi_interactable_object)))

(fn DrawInteractZone
  (bind _result (CallFunction|GetInteractZoneTransform))
  (if (Variables|Interaction|GetdrawInteractionZone)
    (Rendering|Debug|DrawDebugBox (.location _result) (.scale _result) "(R=0.000000,G=1.000000,B=0.079420,A=1.000000)" (.rotation _result) 0.0 0.0)))

(fn GetInteractZoneTransform
  (bind _interactzonetransform (Variables|Interaction|GetinteractZoneTransform))
  (return (Math|Transform|MakeTransform (+ (Transformation|GetActorLocation) (Math|Vector|RotateVector (.location _interactzonetransform) (Math|Rotator|MakeRotator 0.0 0.0 (* (Utilities|Select :Index (Variables|Default|Getdirection) :NewEnumerator0 1.0 :NewEnumerator1 3.0 :NewEnumerator2 0.0 :NewEnumerator3 2.0) 9e+01)))) (.rotation _interactzonetransform) (.scale _interactzonetransform))))

(fn DisableMovement
  (Variables|Default|SetisInDialogue false)
  (Variables|Default|SetisMoving false))

(fn EnableMovement
  (Variables|Default|SetisInDialogue true))